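; Player controller for a mouse-driven game that forwards clicks in the world to grid point handling.
; BeginPlay shows the cursor and enables click events.
; On left mouse release, it deprojects the cursor, line-traces WorldStatic objects and passes the hit actor to CallPointClicked once for each valid GridOuter and GridInner reference.
; Logic to switch the view to the first CameraActor is present but unconnected.
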(event `self.ReceiveBeginPlay`
  (`|ExecutionSequence`
    (:`then_1`
      (set `self.bEnableClickEvents` true)
      (set `self.bShowMouseCursor` true))))

(event `Key|LeftMouseButton`
  (params (Key :type "Key Structure"))
  (bind (_worldlocation _worlddirection) (`self.DeprojectMousePositionToWorld`))
  (:`Released`
    (bind _outhit (`KismetSystemLibrary.LineTraceSingleForObjects` :`Start` _worldlocation :`End` (+ (`PlayerCameraManager.GetCameraLocation` (`GameplayStatics.GetPlayerCameraManager` 0)) (* (`KismetMathLibrary.Normal` (`KismetMathLibrary.Conv_RotatorToVector` (`KismetMathLibrary.Conv_VectorToRotator` _worlddirection))) 10000)) :`ObjectTypes` (`|MakeArray` "ObjectTypeQuery1" :!type "EObjectTypeQuery Enum") :`DrawTime` 10000000.0))
    (`/Engine/EditorBlueprintResources/StandardMacros.IsValid` (`self.GridOuter`)
      (:`Is Valid`
        (bind (_bblockinghit _binitialoverlap _time _distance _location _impactpoint _normal _impactnormal _physmat _hitactor) (`GameplayStatics.BreakHitResult` _outhit))
        (`self.PointClicked` _hitactor))
      (:`Is Not Valid`
        _))
    (`/Engine/EditorBlueprintResources/StandardMacros.IsValid` (`self.GridInner`)
      (:`Is Valid`
        (`self.PointClicked` _hitactor)))))

(fn `UserConstructionScript`)