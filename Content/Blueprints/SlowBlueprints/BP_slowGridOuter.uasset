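; BP_slowGridOuter builds the outer border of a grid around GridInner, with points and planes along all four sides.
; Refresh fills RowThickness from black-material checks on GridInner's first CenterObj, then spawns points at positions from CalculateVectorPoints, which leaves the thickness inputs unused.
; It also fits four border planes to the grid size, reusing one FlipFlop-driven transform for each opposite pair.
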(event `self.ReceiveBeginPlay`
  (`parent.ReceiveBeginPlay`))

(event `self.Refresh`
  (bind _pointscale (`self.PointScale`))
  (bind _pointscale_2 (`self.PointScale`))
  (bind _pointscale_3 (`self.PointScale`))
  (bind _pointscale_4 (`self.PointScale`))
  (bind _returnvalue (`KismetMathLibrary.Conv_IntToDouble` (`self.PointScale`)))
  (bind _returnvalue_2 (`KismetMathLibrary.Conv_IntToDouble` (`self.PointScale`)))
  (`parent.Refresh`)
  (`|ExecutionSequence`
    (:`then_0`
      (`|ExecutionSequence`
        (:`then_0`
          (for _ (range (`self.RowCount`))
            (for _ (range (`self.ColumnCount`))
              (if (== (`PrimitiveComponent.GetMaterial` (`/Game/Blueprints/SlowBlueprints/BaseClasses/BP_slowPointBase.Plane` (`|GetArrayItem` (`/Game/Blueprints/SlowBlueprints/BaseClasses/BP_slowGridBase.CenterObj` (`self.GridInner`)))) 0) "/Game/Materials/MI_Black.MI_Black")
                (`/Engine/EditorBlueprintResources/StandardMacros.IncrementInt` (`self.eachThickness`))))
            (`KismetArrayLibrary.Array_Add` (`self.RowThickness`) (`self.eachThickness`))
            (set `self.eachThickness` 0)))
        (:`then_2`
          (bind _vectorarray (`self.CalculateVectorPoints` (`self.RowCount`) (`self.ColumnCount`) (`self.PointScale`) (`self.RowThickness`) (`self.ColumnThickness`)))
          (bind _output_get (set `self.CenterPoints` _vectorarray))
          (`self.SpawnPointsOnVectorPoints` _output_get (`self.PointClass`)))))
    (:`then_1`
      (`|ExecutionSequence`
        (:`then_0`
          (bind _isa (`/Engine/EditorBlueprintResources/StandardMacros.FlipFlop` :!label _label)
            (:`A`
              _)
            (:`B`
              _))
          ;[1 1 1] Plane Up & Down
          (`SceneComponent.K2_SetRelativeTransform` (select `bool` _isa :`false` (`self.PlaneDown`) :`true` (`self.PlaneUp`) :!type "SceneComponent Object Reference") (`KismetMathLibrary.MakeTransform` (`KismetMathLibrary.MakeVector` (`KismetMathLibrary.Conv_IntToDouble` (- (/ (* (`self.ColumnCount`) _pointscale) 2) (/ _pointscale 2))) (`KismetMathLibrary.Conv_IntToDouble` (`KismetMathLibrary.SelectInt` (* _pointscale -1) (* (`self.RowCount`) (`self.PointScale`)) _isa))) (struct) (/ (`KismetMathLibrary.MakeVector` (`KismetMathLibrary.Conv_IntToDouble` (* (`self.ColumnCount`) _pointscale_2)) (`KismetMathLibrary.Conv_IntToDouble` _pointscale_2) _returnvalue) _returnvalue)) false false))
        (:`then_1`
          (goto _label))
        (:`then_2`
          (bind _isa_2 (`/Engine/EditorBlueprintResources/StandardMacros.FlipFlop` :!label _label_2)
            (:`A`
              _)
            (:`B`
              _))
          ;[1 1 1] Plane Right & Left
          (`SceneComponent.K2_SetRelativeTransform` (select `bool` _isa_2 :`false` (`self.PlaneLeft`) :`true` (`self.PlaneRight`)) (`KismetMathLibrary.MakeTransform` (`KismetMathLibrary.MakeVector` (`KismetMathLibrary.Conv_IntToDouble` (`KismetMathLibrary.SelectInt` (* (`self.ColumnCount`) (`self.PointScale`)) (* (`self.PointScale`) -1) _isa_2)) (`KismetMathLibrary.Conv_IntToDouble` (- (/ (* (`self.RowCount`) _pointscale_4) 2) (/ _pointscale_4 2)))) (struct) (/ (`KismetMathLibrary.MakeVector` (`KismetMathLibrary.Conv_IntToDouble` _pointscale_3) (`KismetMathLibrary.Conv_IntToDouble` (* _pointscale_3 (`self.RowCount`))) _returnvalue_2) _returnvalue_2)) false false))
        (:`then_3`
          (goto _label_2))))))

(fn `CalculateVectorPoints`
  (params (RowCount :type Integer) (ColumnCount :type Integer) (PointScale :type Integer) (RowThickness :type "Array of Integer (by ref)") (ColumnThickness :type "Array of Integer (by ref)"))
  (returns (VectorArray :type "Array of Vector Structure"))
  (locals (Points :type "Array of Vector Structure") (RowCountLoc :type Integer) (ColumnCountLoc :type Integer) (PointScaleLoc :type Integer) (CurrentRow :type Integer) (CurrentColumn :type Integer) (RowThicknessLoc :type "Array of Integer") (ColumnThicknessLoc :type "Array of Integer"))
  (bind _pointscaleloc (`local.PointScaleLoc`))
  (bind _pointscaleloc_2 (`local.PointScaleLoc`))
  (bind _returnvalue (`KismetMathLibrary.Conv_IntToDouble` (* (`local.CurrentRow`) _pointscaleloc_2)))
  (bind _returnvalue_2 (`KismetMathLibrary.Conv_IntToDouble` (* (`local.CurrentColumn`) _pointscaleloc)))
  (set `local.RowCountLoc` RowCount)
  (set `local.ColumnCountLoc` ColumnCount)
  (set `local.PointScaleLoc` PointScale)
  (set `local.RowThicknessLoc` RowThickness)
  (set `local.ColumnThicknessLoc` ColumnThickness)
  (`|ExecutionSequence`
    (:`then_0`
      (for _index (range 2)
        (for _index_2 (range (`local.RowCountLoc`))
          (set `local.CurrentRow` _index_2)
          (`KismetArrayLibrary.Array_Add` (`local.Points`) (`KismetMathLibrary.SelectVector` (`KismetMathLibrary.MakeVector` (`KismetMathLibrary.Conv_IntToDouble` (* _pointscaleloc_2 -1)) _returnvalue) (`KismetMathLibrary.MakeVector` (`KismetMathLibrary.Conv_IntToDouble` (* (`local.ColumnCountLoc`) _pointscaleloc_2)) _returnvalue) (== _index 0))))))
    (:`then_1`
      (for _index_3 (range 2)
        (for _index_4 (range (`local.ColumnCountLoc`))
          (set `local.CurrentColumn` _index_4)
          (`KismetArrayLibrary.Array_Add` (`local.Points`) (`KismetMathLibrary.SelectVector` (`KismetMathLibrary.MakeVector` _returnvalue_2 (`KismetMathLibrary.Conv_IntToDouble` (* _pointscaleloc -1))) (`KismetMathLibrary.MakeVector` _returnvalue_2 (`KismetMathLibrary.Conv_IntToDouble` (* (`local.RowCountLoc`) _pointscaleloc))) (== _index_3 0))))))
    (:`then_2`
      (return (`local.Points`)))))

(fn `UserConstructionScript`
  (`parent.UserConstructionScript`))