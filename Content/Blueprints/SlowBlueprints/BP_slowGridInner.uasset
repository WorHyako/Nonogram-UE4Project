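; Inner grid that spawns clickable point actors in rows and columns and registers itself with the player controller at BeginPlay.
; Refresh computes evenly spaced center points from row, column and scale values, fits the backing plane to them, then spawns the point class on each.
; Clicking a BP_slowPointInner toggles its material between base colour and cyan, while BrushPoints paints the points at given indexes white.
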(event `self.ReceiveBeginPlay`
  (`parent.ReceiveBeginPlay`)
  (bind _asbp_player_controller (cast `/Game/Blueprints/GameManagement/BP_PlayerController` (`GameplayStatics.GetPlayerController` 0)))
  (set `/Game/Blueprints/GameManagement/BP_PlayerController.GridInner` self _asbp_player_controller)
  (add `/Game/Blueprints/GameManagement/BP_PlayerController.PointClicked` _asbp_player_controller (delegate `PointClicked`)))

(event `PointClicked`
  (params (HitActor :type "Actor Object Reference"))
  (`KismetSystemLibrary.PrintString` (`KismetSystemLibrary.GetDisplayName` HitActor))
  (bind _asbp_point_inner (cast `/Game/Blueprints/SlowBlueprints/BP_slowPointInner` HitActor))
  (bind _plane (`/Game/Blueprints/SlowBlueprints/BaseClasses/BP_slowPointBase.Plane` _asbp_point_inner))
  (`PrimitiveComponent.SetMaterial` _plane 0 (select `bool` (== (`PrimitiveComponent.GetMaterial` _plane 0) "/Game/Materials/M_BaseColour.M_BaseColour") :`false` "/Game/Materials/M_BaseColour.M_BaseColour" :`true` "/Game/Materials/MI_Cyan.MI_Cyan" :!type "MaterialInterface Object Reference")))

(event `self.Refresh`
  (bind _array (`|MakeArray` 0))
  (`parent.Refresh`)
  (bind _vectorarray (`self.CalculateVectorPoints` (`self.RowCount`) (`self.ColumnCount`) (`self.PointScale`) _array _array))
  (bind _output_get (set `self.CenterPoints` _vectorarray))
  (`self.SpawnPointsOnVectorPoints` _output_get (`self.PointClass`)))

(event `self.BrushPoints`
  (params (WhiteIndexes :type "Array of Integer (by ref)"))
  (for _array_element WhiteIndexes
    (`PrimitiveComponent.SetMaterial` (`/Game/Blueprints/SlowBlueprints/BaseClasses/BP_slowPointBase.Plane` (`|GetArrayItem` (`self.CenterObj`) _array_element)) 0 "/Game/Materials/MI_White.MI_White")))

(fn `CalculateVectorPoints`
  (params (RowCount :type Integer) (ColumnCount :type Integer) (PointScale :type Integer) (RowThickness :type "Array of Integer (by ref)") (ColumnThickness :type "Array of Integer (by ref)"))
  (returns (VectorArray :type "Array of Vector Structure"))
  (locals (RowCountLoc :type Integer) (ColumnCountLoc :type Integer) (PointScaleLoc :type Integer) (CurrentRow :type Integer) (CurrentColumn :type Integer) (Points :type "Array of Vector Structure"))
  (bind _pointscaleloc (`local.PointScaleLoc`))
  (bind _pointscaleloc_2 (`local.PointScaleLoc`))
  (set `local.RowCountLoc` RowCount)
  (set `local.ColumnCountLoc` ColumnCount)
  (set `local.PointScaleLoc` PointScale)
  (`|ExecutionSequence`
    (:`then_0`
      ;[1 1 1] Center Points
      (for _index (range (`local.RowCountLoc`))
        (set `local.CurrentRow` _index)
        (for _index_2 (range (`local.ColumnCountLoc`))
          (set `local.CurrentColumn` _index_2)
          (`KismetArrayLibrary.Array_Add` (`local.Points`) (`KismetMathLibrary.MakeVector` (`KismetMathLibrary.Conv_IntToDouble` (* (`local.CurrentColumn`) _pointscaleloc)) (`KismetMathLibrary.Conv_IntToDouble` (* _pointscaleloc (`local.CurrentRow`))))))))
    (:`then_1`
      ;[1 1 1] Plane
      (`SceneComponent.K2_SetRelativeTransform` (`self.Plane`) (`KismetMathLibrary.MakeTransform` (/ (`|GetArrayItem` (`local.Points`) (- (`KismetArrayLibrary.Array_Length` (`local.Points`)) 1)) 2) (struct) (/ (`KismetMathLibrary.MakeVector` (`KismetMathLibrary.Conv_IntToDouble` (* (`local.ColumnCountLoc`) _pointscaleloc_2)) (`KismetMathLibrary.Conv_IntToDouble` (* (`local.RowCountLoc`) _pointscaleloc_2)) 1.0) 100.0)) false false))
    (:`then_2`
      (return (`local.Points`)))))

(fn `UserConstructionScript`
  (`parent.UserConstructionScript`))