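; BP_SlowGridManager coordinates an inner and outer point grid and frames them with a camera.
; RefreshGridManager takes dimensions from an optional TextureReader, clamps size and point scale, then pushes them to both grids, refreshing and centering each.
; It places the camera looking down at a height based on the larger dimension.
; BeginPlay is empty; the delayed refresh and brushing of the texture's white pixels are disconnected.
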(event `RefreshGridManager`
  (bind _texturereader (`self.TextureReader`))
  (bind _pointscale (`self.PointScale`))
  (bind _returnvalue (/ _pointscale 2))
  (`|ExecutionSequence`
    (:`then_0`
      (`/Engine/EditorBlueprintResources/StandardMacros.IsValid` _texturereader
        (:`Is Valid`
          (set `self.RowCount` (`TextureReader._textureSizeX` _texturereader))
          (set `self.ColumnCount` (`TextureReader._textureSizeY` _texturereader)))))
    (:`then_1`
      (if (< (`self.PointScale`) 10)
        (set `self.PointScale` 10))
      (if (< (`self.RowCount`) 1)
        (set `self.RowCount` 1))
      (if (< (`self.ColumnCount`) 1)
        (set `self.ColumnCount` 1))
      (if (> (`self.RowCount`) 50)
        (set `self.RowCount` 50))
      (if (> (`self.ColumnCount`) 50)
        (set `self.ColumnCount` 50)))
    (:`then_2`
      (for _array_element (`|MakeArray` (`self.GridInner`) (`self.GridOuter`) :!type "/Game/Blueprints/SlowBlueprints/BaseClasses/BP_slowGridBase Object Reference")
        (`/Engine/EditorBlueprintResources/StandardMacros.IsValid` _array_element
          (:`Is Valid`
            (set `/Game/Blueprints/SlowBlueprints/BaseClasses/BP_slowGridBase.RowCount` (`self.RowCount`) _array_element)
            (set `/Game/Blueprints/SlowBlueprints/BaseClasses/BP_slowGridBase.ColumnCount` (`self.ColumnCount`) _array_element)
            (set `/Game/Blueprints/SlowBlueprints/BaseClasses/BP_slowGridBase.PointScale` (`self.PointScale`) _array_element)
            (`/Game/Blueprints/SlowBlueprints/BaseClasses/BP_slowGridBase.Refresh` _array_element)
            (`self.K2_SetActorLocation` _array_element (`KismetMathLibrary.MakeVector` (`KismetMathLibrary.Conv_IntToDouble` (+ (/ (* (`self.ColumnCount`) _pointscale -1) 2) _returnvalue)) (`KismetMathLibrary.Conv_IntToDouble` (+ _returnvalue (/ (* _pointscale (`self.RowCount`) -1) 2)))) false false)))))
    (:`then_3`
      (`/Engine/EditorBlueprintResources/StandardMacros.IsValid` (`self.Camera`)
        (:`Is Valid`
          (`self.K2_SetActorTransform` (`self.Camera`) (`KismetMathLibrary.MakeTransform` (`KismetMathLibrary.MakeVector` 0.0 0.0 (* (`KismetMathLibrary.Conv_IntToDouble` (`KismetMathLibrary.SelectInt` (/ (* (`self.RowCount`) (`self.PointScale`)) 2) (/ (* (`self.ColumnCount`) (`self.PointScale`)) 2) (> (`self.RowCount`) (`self.ColumnCount`)))) 1.4)) (struct :`Pitch` -90.0 :`Yaw` -90.0 :`Roll` -90.0)) false false))))))

(event `self.ReceiveBeginPlay`)

(fn `UserConstructionScript`)