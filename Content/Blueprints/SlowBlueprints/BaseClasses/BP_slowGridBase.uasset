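; BP_slowGridBase is a base grid actor that spawns and manages BP_slowPointBase actors at supplied positions.
; SpawnPointsOnVectorPoints places a point actor at each XY on a fixed height, attaches it to the grid and stores it in CenterObj.
; Refresh detaches and destroys stored points, clears both arrays and forces garbage collection.
; CalculateVectorPoints and BrushPoints are empty here, leaving layout and brush logic unimplemented.
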(event `BrushPoints`
  (params (WhiteIndexes :type "Array of Integer")))

(event `Refresh`
  (for _array_element (`self.CenterObj`)
    (`/Engine/EditorBlueprintResources/StandardMacros.IsValid` _array_element
      (:`Is Valid`
        (`self.K2_DetachFromActor` _array_element "KeepRelative" "KeepRelative" "KeepRelative")
        (`self.K2_DestroyActor` _array_element))))
  (`KismetArrayLibrary.Array_Clear` (`self.CenterObj`))
  (`KismetArrayLibrary.Array_Clear` (`self.CenterPoints`))
  (`KismetSystemLibrary.CollectGarbage`))

(event `self.ReceiveBeginPlay`)

(event `self.ReceiveEndPlay`
  (params (EndPlayReason :type "EEndPlayReason Enum" :default "Destroyed"))
  (`KismetArrayLibrary.Array_Clear` (`self.CenterPoints`))
  (`KismetArrayLibrary.Array_Clear` (`self.CenterObj`)))

(fn `CalculateVectorPoints`
  (params (RowCount :type Integer) (ColumnCount :type Integer) (PointScale :type Integer) (RowThickness :type "Array of Integer") (ColumnThickness :type "Array of Integer"))
  (returns (VectorArray :type "Array of Vector Structure"))
  (return))

(fn `SpawnPointsOnVectorPoints`
  (params (VectorPoints :type "Array of Vector Structure") (PointClass :type "Actor Class Reference"))
  (locals (Points :type "Array of Vector Structure"))
  (bind _output_get (set `local.Points` VectorPoints))
  (for _index (range (`KismetArrayLibrary.Array_Length` _output_get))
    (bind (_output_x _output_y) (`KismetMathLibrary.BreakVector` (`|GetArrayItem` (`local.Points`) _index)))
    (bind _returnvalue (`|SpawnActorFromClass` PointClass (`KismetMathLibrary.MakeTransform` (`KismetMathLibrary.MakeVector` _output_x _output_y 10.0)) "Undefined" "OverrideRootScale" self null))
    (`/Engine/EditorBlueprintResources/StandardMacros.IsValid` _returnvalue
      (:`Is Valid`
        (bind _asbp_point_base (cast `/Game/Blueprints/SlowBlueprints/BaseClasses/BP_slowPointBase` _returnvalue))
        (`self.K2_AttachToActor` _asbp_point_base self "None" "KeepRelative" "KeepRelative" "KeepRelative" true)
        (`KismetArrayLibrary.Array_Add` (`self.CenterObj`) _asbp_point_base))))
  (return))

(fn `UserConstructionScript`)