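; BP_GridGenerate is an actor that builds a flat, clickable grid of square cells at BeginPlay.
; Nested row and column loops create each cell as its own collision-enabled procedural mesh section, sized and placed by PointScale.
; A FlipFlop alternates cyan and black materials in creation order without resetting per row, then the section count is stored.
; Clicking the mesh prints the deprojected mouse world location, not the clicked cell.
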(event `self.ReceiveBeginPlay`
  (bind _drawgrid (`self.DrawGrid`))
  (bind _pointscale (`self.PointScale`))
  (bind _pointscale_2 (`self.PointScale`))
  (bind _pointscale_3 (`self.PointScale`))
  (bind _pointscale_4 (`self.PointScale`))
  (bind _returnvalue (/ _pointscale_4 2.0))
  (bind _returnvalue_2 (/ _pointscale 2.0))
  (bind _returnvalue_3 (/ _pointscale_2 2.0))
  (bind _returnvalue_4 (/ _pointscale_3 2.0))
  (bind _returnvalue_5 (+ (* (`self.ColumnCount`) (`self.CurrentRow`)) (`self.CurrentColumn`)))
  (`|ExecutionSequence`
    (:`then_1`
      (for _index (range (`self.RowCount`))
        (set `self.CurrentRow` _index)
        (for _index_2 (range (`self.ColumnCount`))
          (`KismetArrayLibrary.Array_Clear` (`self.Vertex`))
          (set `self.CurrentColumn` _index_2)
          (`|ExecutionSequence`
            (:`then_0`
              (`|ExecutionSequence`
                (:`then_0`
                  (`KismetArrayLibrary.Array_Add` (`self.Vertex`) (`KismetMathLibrary.MakeVector` (- (* (`self.CurrentColumn`) _pointscale) _returnvalue_2) (- (* (`self.CurrentRow`) _pointscale) _returnvalue_2))))
                (:`then_1`
                  (`KismetArrayLibrary.Array_Add` (`self.Vertex`) (`KismetMathLibrary.MakeVector` (+ (* (`self.CurrentColumn`) _pointscale_2) _returnvalue_3) (- (* (`self.CurrentRow`) _pointscale_2) _returnvalue_3))))
                (:`then_2`
                  (`KismetArrayLibrary.Array_Add` (`self.Vertex`) (`KismetMathLibrary.MakeVector` (+ (* (`self.CurrentColumn`) _pointscale_3) _returnvalue_4) (+ _returnvalue_4 (* (`self.CurrentRow`) _pointscale_3)))))
                (:`then_3`
                  (`KismetArrayLibrary.Array_Add` (`self.Vertex`) (`KismetMathLibrary.MakeVector` (- (* (`self.CurrentColumn`) _pointscale_4) _returnvalue) (+ _returnvalue (* (`self.CurrentRow`) _pointscale_4)))))))
            (:`then_1`
              (`ProceduralMeshComponent.CreateMeshSection_LinearColor` :`self` _drawgrid :`SectionIndex` _returnvalue_5 :`Vertices` (`self.Vertex`) :`Triangles` (`|MakeArray` 2 1 0 3 2 0) :`bCreateCollision` true)
              (bind _isa (`/Engine/EditorBlueprintResources/StandardMacros.FlipFlop`)
                (:`A`
                  _)
                (:`B`
                  _))
              (`PrimitiveComponent.SetMaterial` _drawgrid _returnvalue_5 (select `bool` _isa :`false` "/Game/Materials/MI_Black.MI_Black" :`true` "/Game/Materials/MI_Cyan.MI_Cyan" :!type "MaterialInterface Object Reference")))))))
    (:`then_2`
      (set `self.SectionNum` (`ProceduralMeshComponent.GetNumSections` (`self.DrawGrid`))))))

(event `self.DrawGrid.OnClicked`
  (params (TouchedComponent :type "PrimitiveComponent Object Reference") (ButtonPressed :type "Key Structure"))
  (cast `ProceduralMeshComponent` TouchedComponent)
  (`KismetSystemLibrary.PrintString` (`KismetStringLibrary.Conv_VectorToString` (`PlayerController.DeprojectMousePositionToWorld` (`GameplayStatics.GetPlayerController` 0)))))

(fn `UserConstructionScript`)