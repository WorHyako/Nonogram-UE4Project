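; BP_Grid is a grid actor that lays out center-point markers from configurable row and column counts.
; The Construction Script resets out-of-range counts to one, then adds a small static mesh component per cell, spaced by PointScale.
; BeginPlay destroys those meshes and clears their array, so the markers do not persist into play.
; Wall building and the spawning of BP_slowPointBase actors at each point are present but disconnected.
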(event `self.ReceiveBeginPlay`
  (bind _centerpointscomponents (`self.CenterPointsComponents`))
  (`|ExecutionSequence`
    (:`then_0`
      (for _array_element _centerpointscomponents
        _)
      (for _array_element_2 _centerpointscomponents
        (`ActorComponent.K2_DestroyComponent` _array_element_2))
      (`KismetArrayLibrary.Array_Clear` _centerpointscomponents))))

(fn `UserConstructionScript`
  (locals (WallTransform :type "Transform Structure") (CurrentRowIndex :type Integer) (CurrentColumnIndex :type Integer))
  (bind _columncount (`self.ColumnCount`))
  (bind _rowcount (`self.RowCount`))
  (bind _pointscale (`self.PointScale`))
  (bind _rowcount_2 (`self.RowCount`))
  (bind _columncount_2 (`self.ColumnCount`))
  (`|ExecutionSequence`
    (:`then_0`
      (`KismetArrayLibrary.Array_Clear` (`self.CenterPointsComponents`))
      (`KismetArrayLibrary.Array_Clear` (`self.WallComponents`)))
    (:`then_1`
      (if (or (< _rowcount 1) (> _rowcount (`self.MaxRowCount`)) (< _columncount 1) (> _columncount (`self.MaxColumnCount`)))
        (if (or (< _rowcount_2 1) (> _rowcount_2 (`self.MaxRowCount`)))
          (set `self.RowCount` 1))
        (if (or (< _columncount_2 1) (> _columncount_2 (`self.MaxColumnCount`)))
          (set `self.ColumnCount` 1)))
      (for _index (range (`self.RowCount`))
        (set `local.CurrentRowIndex` _index)
        (for _index_2 (range (`self.ColumnCount`))
          (set `local.CurrentColumnIndex` _index_2)
          ;[1 1 1] Center Point
          (bind _returnvalue (`AddComponent|NODE_AddStaticMeshComponent-0` :`bManualAttachment` true :`RelativeTransform` (`KismetMathLibrary.MakeTransform` (`KismetMathLibrary.MakeVector` (* (`local.CurrentColumnIndex`) _pointscale) (* (`local.CurrentRowIndex`) _pointscale)) (struct) (0.2 0.2 0.2))))
          (bind _returnvalue_2 (`KismetArrayLibrary.Array_Add` (`self.CenterPointsComponents`) _returnvalue))
          (`SceneComponent.K2_AttachToComponent` _returnvalue (`self.DefaultSceneRoot`) "None" "KeepRelative" "KeepRelative" "KeepRelative" true))))))